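; Game mode for a frog game that runs the level as numbered sequences, starting with an intro.
; On BeginPlay it has placed spawners, cameras, end ways, collectibles and spawn/weather points register themselves, then advances the sequence.
; Each later sequence repositions the spawner, swaps Niagara rain and wind, and blends the camera view.
; Once past the intro, Tick drives frog spawning and moves all registered frogs centrally.
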(event `self.ReceiveBeginPlay`
  (bind _allelementsareregister (`self.RegisterAllElements`))
  (if _allelementsareregister
    (`self.GoNextSequence`)))

(event `self.ReceiveTick`
  (params (DeltaSeconds :type "Float (single-precision)"))
  (bind _result (`self.WasIntroPlayed`))
  (if _result
    (`/Game/BP_Spawner.SpawnEntity` (`self.Spawner`) DeltaSeconds)
    (for _array_element (`self.Frogs`)
      (`/Game/Frog/BP_Frog.MoveFrog` _array_element DeltaSeconds))))

(fn `AddItemToCollected`
  (params (NewMeshItem :type "StaticMesh Object Reference"))
  (if (`KismetSystemLibrary.IsValid` NewMeshItem)
    (`KismetArrayLibrary.Array_AddUnique` (`self.MeshsCollected`) NewMeshItem)))

(fn `AutoRegisterFrog`
  (params (NewFrog :type "/Game/Frog/BP_Frog Object Reference"))
  (if (`KismetSystemLibrary.IsValid` NewFrog)
    (`KismetArrayLibrary.Array_AddUnique` (`self.Frogs`) NewFrog)))

(fn `CollectOldSequenceWeatherActors`
  (bind _currentsequenceweatheractors (`self.CurrentSequenceWeatherActors`))
  (for _array_element _currentsequenceweatheractors
    (if (`KismetSystemLibrary.IsValid` _array_element)
      (`KismetArrayLibrary.Array_AddUnique` (`self.OldSequenceWeatherActors`) _array_element)
      (bind _returnvalue (`KismetArrayLibrary.Array_RemoveItem` _currentsequenceweatheractors _array_element))
      (if _returnvalue
        (if (not (== (`KismetArrayLibrary.Array_Length` _currentsequenceweatheractors) 0))
          (`KismetSystemLibrary.PrintText` "Sequence error, one or more elements could not be remove from current sequence pool."))
        (return)
        (else
          (`KismetSystemLibrary.PrintText` (`KismetTextLibrary.Conv_StringToText` (`KismetStringLibrary.Concat_StrStr` "Sequence error, one elements could not be place in old object pool :" (`KismetSystemLibrary.GetObjectName` _array_element))))))
      (else
        (`KismetSystemLibrary.PrintText` "Sequence error, invalid weather element." true true (struct :`R` 1.0 :`B` 0.05661 :`A` 1.0) 5.0)))))

(fn `DestroyOldSequenceWeatherActors`
  (bind _oldsequenceweatheractors (`self.OldSequenceWeatherActors`))
  (for _array_element _oldsequenceweatheractors
    (if (`KismetSystemLibrary.IsValid` _array_element)
      (`self.K2_DestroyActor` _array_element)))
  (`KismetArrayLibrary.Array_Clear` _oldsequenceweatheractors)
  (return))

(fn `DisplayErrorRegister`
  (params (ObjectName :type String))
  (`KismetSystemLibrary.PrintText` (`KismetTextLibrary.Conv_StringToText` (`KismetStringLibrary.Concat_StrStr` "Error register : " ObjectName)))
  (return))

(fn `EnableRainToSequencePosition`
  (params (TargetSequenceID :type Integer))
  (bind _output (`|GetArrayItem` (`self.RainPoints`) TargetSequenceID))
  (bind (_returnvalue_location _returnvalue_rotation _returnvalue_scale) (`KismetMathLibrary.BreakTransform` (`self.GetTransform` _output)))
  (if (`KismetSystemLibrary.IsValid` _output)
    (bind _returnvalue (`NiagaraFunctionLibrary.SpawnSystemAtLocation` (`/Game/BP_RainPoint.TargetNiagara` _output) _returnvalue_location _returnvalue_rotation _returnvalue_scale false true "None" false))
    (if (`KismetSystemLibrary.IsValid` _returnvalue)
      (`KismetArrayLibrary.Array_AddUnique` (`self.CurrentSequenceWeatherActors`) (`ActorComponent.GetOwner` _returnvalue))
      (return)
      (else
        (`KismetSystemLibrary.PrintText` (`KismetTextLibrary.Conv_StringToText` (`KismetStringLibrary.Concat_StrStr` "Sequence error, unable to spawn Rain Niagara system at point :" (`KismetSystemLibrary.GetObjectName` _output))) true true (struct :`G` 0.66 :`B` 1.0 :`A` 1.0) 5.0)
        (return)))))

(fn `EnableWindToSequencePosition`
  (params (TargetSequenceID :type Integer))
  (for _array_element (`self.WindPoints`)
    (if (`KismetSystemLibrary.IsValid` _array_element)
      (if (== (`/Game/BP_WindPoint.AssociatedSequenceIndex` _array_element) TargetSequenceID)
        (bind (_returnvalue_location _returnvalue_rotation _returnvalue_scale) (`KismetMathLibrary.BreakTransform` (`self.GetTransform` _array_element)))
        (bind _returnvalue (`NiagaraFunctionLibrary.SpawnSystemAtLocation` (`/Game/BP_WindPoint.TargetNiagara` _array_element) _returnvalue_location _returnvalue_rotation _returnvalue_scale false true "None" false))
        (if (`KismetSystemLibrary.IsValid` _returnvalue)
          (`KismetArrayLibrary.Array_AddUnique` (`self.CurrentSequenceWeatherActors`) (`ActorComponent.GetOwner` _returnvalue))
          (else
            (`KismetSystemLibrary.PrintText` (`KismetTextLibrary.Conv_StringToText` (`KismetStringLibrary.Concat_StrStr` "Sequence error, unable to spawn Wing Niagara system at point :" (`KismetSystemLibrary.GetObjectName` _array_element))))
            (return))))
      (else
        (`KismetSystemLibrary.PrintText` "Sequence error, unable to get WindPoint to spawn Wind Niagara system")
        (return))))
  (return))

(fn `GoNextSequence`
  (bind _currentsequenceindex (`self.CurrentSequenceIndex`))
  (bind _currentsequenceindex_2 (`self.CurrentSequenceIndex`))
  (if (`self.IsAlreadyRunningNewSequence`)
    (return)
    (else
      (set `self.IsAlreadyRunningNewSequence` true)
      (bind _result (`/Engine/EditorBlueprintResources/StandardMacros.IncrementInt` _currentsequenceindex)
        (:`  `
          (bind _output_get (set `self.CurrentSequenceIndex` _result))
          (if (== _output_get 0)
            (`self.MoveCameraToSequencePosition` _currentsequenceindex)
            (set `self.IsAlreadyRunningNewSequence` false)
            (return)
            (else
              (`self.CollectOldSequenceWeatherActors`)
              (`self.SetupSpawnerToSequencePosition` _currentsequenceindex_2)
              (`self.EnableRainToSequencePosition` _currentsequenceindex_2)
              (`self.EnableWindToSequencePosition` _currentsequenceindex_2)
              (`self.MoveCameraToSequencePosition` _currentsequenceindex_2 (`self.CameraSpeed`))
              (`self.DestroyOldSequenceWeatherActors`)
              (set `self.IsAlreadyRunningNewSequence` false)
              (return))))))))

(fn `MoveCameraToSequencePosition`
  (params (TargetSequenceID :type Integer) (BlendTime :type "Float (double-precision)"))
  (bind _output (`|GetArrayItem` (`self.SequenceCameras`) TargetSequenceID))
  (if (`KismetSystemLibrary.IsValid` _output)
    (`PlayerController.SetViewTargetWithBlend` (`GameplayStatics.GetPlayerController` 0) _output BlendTime "VTBlend_Cubic" 0.0 true)))

(fn `RegisterAllElements`
  (returns (AllElementsAreRegister :type Boolean))
  (bind _outactors (`GameplayStatics.GetAllActorsOfClass` "/Game/BP_Spawner.BP_Spawner_C"))
  (for _array_element _outactors
    (`/Game/BP_Spawner.Register` _array_element self))
  (bind _outactors_2 (`GameplayStatics.GetAllActorsOfClass` "/Game/BP_SequenceCamera.BP_SequenceCamera_C"))
  (for _array_element_2 _outactors_2
    (`/Game/BP_SequenceCamera.Register` _array_element_2 self))
  (bind _outactors_3 (`GameplayStatics.GetAllActorsOfClass` "/Game/BP_EndWay.BP_EndWay_C"))
  (for _array_element_3 _outactors_3
    (if (not (`/Game/BP_EndWay.IsJustKill` _array_element_3))
      (`/Game/BP_EndWay.Register` _array_element_3 self)))
  (bind _outactors_4 (`GameplayStatics.GetAllActorsOfClass` "/Game/Collectible/BP_Collectible.BP_Collectible_C"))
  (for _array_element_4 _outactors_4
    (`/Game/Collectible/BP_Collectible.Register` _array_element_4 self))
  (bind _outactors_5 (`GameplayStatics.GetAllActorsOfClass` "/Game/BP_SpawnerPoint.BP_SpawnerPoint_C"))
  (for _array_element_5 _outactors_5
    (`/Game/BP_SpawnerPoint.Register` _array_element_5 self))
  (bind _outactors_6 (`GameplayStatics.GetAllActorsOfClass` "/Game/BP_RainPoint.BP_RainPoint_C"))
  (for _array_element_6 _outactors_6
    (`/Game/BP_RainPoint.Register` _array_element_6 self))
  (bind _outactors_7 (`GameplayStatics.GetAllActorsOfClass` "/Game/BP_WindPoint.BP_WindPoint_C"))
  (for _array_element_7 _outactors_7
    (`/Game/BP_WindPoint.Register` _array_element_7 self))
  (return true))

(fn `SetupSpawnerToSequencePosition`
  (params (TargetSequenceID :type Integer))
  (bind _spawner (`self.Spawner`))
  (bind _output (`|GetArrayItem` (`self.SpawnerPoints`) TargetSequenceID))
  (bind _associatedstartingspline (`/Game/BP_SpawnerPoint.AssociatedStartingSpline` _output))
  (if (`KismetSystemLibrary.IsValid` _output)
    (if (`KismetSystemLibrary.IsValid` (`self.Spawner`))
      (if (`KismetSystemLibrary.IsValid` _associatedstartingspline)
        (set `/Game/BP_Spawner.StartingSpline` _associatedstartingspline _spawner)
        (set `/Game/BP_Spawner.CurrentSpawnerPoint` _output _spawner)
        (return)
        (else
          (`KismetSystemLibrary.PrintText` (`KismetTextLibrary.Conv_StringToText` (`KismetStringLibrary.Concat_StrStr` "Sequence error, no or invalid StartingSpline for the sequence :" (`KismetStringLibrary.Conv_IntToString` TargetSequenceID))))))
      (else
        (`KismetSystemLibrary.PrintText` (`KismetTextLibrary.Conv_StringToText` (`KismetStringLibrary.Concat_StrStr` "Sequence error, no or invalid Spawner for the sequence :" (`KismetStringLibrary.Conv_IntToString` TargetSequenceID))))))
    (else
      (`KismetSystemLibrary.PrintText` (`KismetTextLibrary.Conv_StringToText` (`KismetStringLibrary.Concat_StrStr` "Sequence error, no or invalid SpawnerPoint for the sequence :" (`KismetStringLibrary.Conv_IntToString` TargetSequenceID)))))))

(fn `UnregisterFrog`
  (params (FrogToRemove :type "/Game/Frog/BP_Frog Object Reference"))
  (returns (`Success status` :type Boolean))
  (bind _returnvalue (`KismetArrayLibrary.Array_RemoveItem` (`self.Frogs`) FrogToRemove))
  (return _returnvalue))

(fn `UserConstructionScript`)

(fn `WasIntroPlayed`
  (returns (Result :type Boolean))
  (return (> (`self.CurrentSequenceIndex`) 0)))