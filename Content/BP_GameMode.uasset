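; Game mode that drives a frog game through a fixed-interval game cycle.
; BeginPlay starts a looping timer at GameCycleSpeed, and each tick calls UpdateSpawner and then UpdateFrogs, both currently empty stubs.
; RegisterSpawner stores a single valid spawner reference, while RegisterFrog adds valid frogs to a unique list.
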(event `self.ReceiveBeginPlay`
  (`KismetSystemLibrary.K2_SetTimerDelegate` (delegate `GameCycle`) (`self.GameCycleSpeed`) true))

(event `GameCycle`
  (`self.UpdateSpawner`)
  (`self.UpdateFrogs`))

(fn `RegisterFrog`
  (params (NewFrog :type "/Game/Frog/BP_Frog Object Reference"))
  (if (`KismetSystemLibrary.IsValid` NewFrog)
    (`KismetArrayLibrary.Array_AddUnique` (`self.Frogs`) NewFrog)))

(fn `RegisterSpawner`
  (params (NewSpawner :type "/Game/BP_Spawner Object Reference"))
  (if (`KismetSystemLibrary.IsValid` NewSpawner)
    (set `self.Spawner` NewSpawner)))

(fn `UpdateFrogs`)

(fn `UpdateSpawner`)

(fn `UserConstructionScript`)