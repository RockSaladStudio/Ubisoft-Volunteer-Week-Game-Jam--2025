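; BP_Interactable is an interactable object, apparently a base, that reacts to cursor hover and tracks whether it is being interacted with.
; On BeginPlay it binds cursor enter and exit events, which call OnMaterialChange with the hover state regardless of CanBeInteracted.
; Interact_Event sets Interacting only when CanBeInteracted is true, and StopInteract_Event clears it.
; OnMaterialChange, the construction script and the hover CanBeInteracted branches are empty.
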(event `self.ReceiveBeginPlay`
  (add `self.CursorOverEnter` (delegate `CursorOverEnter_Event`))
  (add `self.CursorOverExit` (delegate `CursorOverExit_Event`)))

(event `CursorOverEnter_Event`
  (`self.OnMaterialChange` true)
  (if (`self.bCanBeInteracted`)
    _))

(event `CursorOverExit_Event`
  (`self.OnMaterialChange` false)
  (if (`self.bCanBeInteracted`)
    _))

(event `Interact_Event`
  (if (`self.bCanBeInteracted`)
    (set `self.bInteracting` true)))

(event `StopInteract_Event`
  (set `self.bInteracting` false))

(fn `OnMaterialChange`
  (params (bIsHovered :type Boolean)))

(fn `UserConstructionScript`)