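; BP_Way is a spline-driven path actor that lays a repeated static mesh along its spline in the Construction Script.
; When generation is allowed, it adds one collidable spline mesh per section, with section length optionally derived from the actor's X scale.
; Start and end helpers sample the spline by distance and clamp tangents to section length to fit each segment.
; IsFullLengh limits output to whole sections; otherwise an extra section covers the remainder.
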(fn `GetEndPosTangent`
  (params (Index :type Integer))
  (returns (Position :type "Vector Structure") (Tangent :type "Vector Structure"))
  (bind _spline (`self.Spline`))
  (bind _sectionlengh (`self.SectionLengh`))
  (bind _returnvalue (* (+ Index 1) _sectionlengh))
  (return (`SplineComponent.GetLocationAtDistanceAlongSpline` _spline _returnvalue "Local") (`KismetMathLibrary.ClampVectorSize` (`SplineComponent.GetTangentAtDistanceAlongSpline` _spline _returnvalue "Local") 0.0 _sectionlengh)))

(fn `GetStartPosTangent`
  (params (Index :type Integer))
  (returns (Position :type "Vector Structure") (Tangent :type "Vector Structure"))
  (bind _spline (`self.Spline`))
  (bind _sectionlengh (`self.SectionLengh`))
  (bind _returnvalue (* Index _sectionlengh))
  (return (`SplineComponent.GetLocationAtDistanceAlongSpline` _spline _returnvalue "Local") (`KismetMathLibrary.ClampVectorSize` (`SplineComponent.GetTangentAtDistanceAlongSpline` _spline _returnvalue "Local") 0.0 _sectionlengh)))

(fn `UserConstructionScript`
  (bind _returnvalue_x (`KismetMathLibrary.BreakVector` (`self.GetActorScale3D`)))
  (bind _loopindex (`self.LoopIndex`))
  (bind _spline (`self.Spline`))
  (if (`self.AllowGeneration`)
    (if (`self.Scalable`)
      (set `self.SectionLengh` (* _returnvalue_x 100.0)))
    (if (`self.IsFullLengh`)
      (for _index (range (`KismetMathLibrary.FTrunc` (/ (`SplineComponent.GetSplineLength` _spline) (`self.SectionLengh`))))
        (set `self.LoopIndex` _index)
        (bind _returnvalue (`AddComponent|NODE_AddSplineMeshComponent-1` :!label _label))
        (`StaticMeshComponent.SetStaticMesh` _returnvalue (`self.SplineMesh`))
        (`SplineMeshComponent.SetForwardAxis` _returnvalue "X" true)
        (bind (_position _tangent) (`self.GetStartPosTangent` _loopindex))
        (bind (_position_2 _tangent_2) (`self.GetEndPosTangent` _loopindex))
        (`SplineMeshComponent.SetStartAndEnd` _returnvalue _position _tangent _position_2 _tangent_2 true)
        (`PrimitiveComponent.SetCollisionEnabled` _returnvalue "QueryAndPhysics"))
      (else
        (for _index_2 (range (+ (`KismetMathLibrary.FTrunc` (/ (`SplineComponent.GetSplineLength` _spline) (`self.SectionLengh`))) 1))
          (set `self.LoopIndex` _index_2)
          (goto _label))))))