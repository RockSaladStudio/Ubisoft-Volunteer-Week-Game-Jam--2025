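; Frog actor that travels along a spline and can carry a collected mesh item on a socket.
; InitFrog registers it with BP_FrogGameMode, updates its spawner's count and attaches the first collected mesh, if any.
; MoveFrog drives a timeline at speed over spline length, easing location and rotation toward the path until close enough to snap.
; KillFrog decrements that count, returns any carried mesh to the game mode, then unregisters and destroys the frog.
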(event `MoveFrog`
  (params (DeltaTime :type "Float (double-precision)"))
  (bind _returnvalue (`self.K2_GetActorRotation`))
  (bind _returnvalue_2 (`self.K2_GetActorLocation`))
  (bind _returnvalue_3 (`GameplayStatics.GetWorldDeltaSeconds`))
  (bind _spline (`/Game/BP_Way.Spline` (`self.SplineToFollow`)))
  (if (and (`KismetSystemLibrary.IsValid` (`self.SplineToFollow`)) (`KismetSystemLibrary.IsValid` (`self.T_Move`)))
    (bind _playrate (`self.GetPlayRate`))
    (`TimelineComponent.SetPlayRate` (`self.T_Move`) _playrate)
    (bind (_direction _move_track) (`Timeline|T_Move`)
      (:`Update`
        (if (`KismetSystemLibrary.IsValid` (`self.SplineToFollow`))
          (bind _interpspeed (`self.GetInterpSplineSpeed`))
          (bind _returnvalue_4 (`KismetMathLibrary.Lerp` 0.0 (`SplineComponent.GetSplineLength` _spline) _move_track))
          (bind _returnvalue_5 (`SplineComponent.GetLocationAtDistanceAlongSpline` _spline _returnvalue_4 "World"))
          (bind _returnvalue_6 (`SplineComponent.GetRotationAtDistanceAlongSpline` _spline _returnvalue_4 "World"))
          (bind (_returnvalue_roll _returnvalue_pitch _returnvalue_yaw) (`KismetMathLibrary.BreakRotator` (`KismetMathLibrary.NormalizedDeltaRotator` _returnvalue_6 _returnvalue)))
          (`self.K2_SetActorLocationAndRotation` (select `bool` (< (`KismetMathLibrary.VSize` (- _returnvalue_5 _returnvalue_2)) 25.0) :`false` (`KismetMathLibrary.VInterpTo` _returnvalue_2 _returnvalue_5 _returnvalue_3 _interpspeed) :`true` _returnvalue_5) (`KismetMathLibrary.SelectRotator` _returnvalue_6 (`KismetMathLibrary.RInterpTo` _returnvalue _returnvalue_6 _returnvalue_3 _interpspeed) (and (< (`KismetMathLibrary.Abs` _returnvalue_roll) 1.0) (< (`KismetMathLibrary.Abs` _returnvalue_pitch) 1.0) (< (`KismetMathLibrary.Abs` _returnvalue_yaw) 1.0)))))))))

(event `self.ReceiveActorBeginOverlap`
  (params (OtherActor :type "Actor Object Reference"))
  (`KismetSystemLibrary.PrintText` (`KismetTextLibrary.Conv_StringToText` (`KismetSystemLibrary.GetObjectName` OtherActor))))

(fn `AddStaticMeshItem`
  (params (MeshToAdd :type "StaticMesh Object Reference"))
  (returns (ItemWasAdd :type Boolean))
  (if (`self.IsCarryItem`)
    (return false)
    (elif (`SceneComponent.DoesSocketExist` (`self.FrogMesh`) (`self.ItemSocketName`))
      (bind _returnvalue (`AddComponent|NODE_AddStaticMeshComponent-0`))
      (if (`KismetSystemLibrary.IsValid` _returnvalue)
        (`StaticMeshComponent.SetStaticMesh` _returnvalue MeshToAdd)
        (`PrimitiveComponent.SetCollisionEnabled` _returnvalue "NoCollision")
        (bind _returnvalue_2 (`SceneComponent.K2_AttachToComponent` _returnvalue (`self.FrogMesh`) (`self.ItemSocketName`) "SnapToTarget" "SnapToTarget" "KeepRelative" true))
        (if _returnvalue_2
          (set `self.IsCarryItem` true)
          (set `self.TransportedMesh` MeshToAdd)
          (bind _asbp_frog_game_mode (cast `/Game/BP_FrogGameMode` (`GameplayStatics.GetGameMode`)))
          (`KismetArrayLibrary.Array_RemoveItem` (`/Game/BP_FrogGameMode.MeshsCollected` _asbp_frog_game_mode) MeshToAdd)
          (return true))))))

(fn `GetInterpSplineSpeed`
  (returns (InterpSpeed :type "Float (double-precision)"))
  (return (/ (`self.FrogSpeed`) 30.0)))

(fn `GetPlayRate`
  (returns (PlayRate :type "Float (double-precision)"))
  (return (/ (`self.FrogSpeed`) (`SplineComponent.GetSplineLength` (`/Game/BP_Way.Spline` (`self.SplineToFollow`))))))

(fn `InitFrog`
  (params (SpawnerOrigin :type "/Game/BP_Spawner Object Reference") (SplineToFollow :type "/Game/BP_Way Object Reference"))
  (bind _spawnerorigin (`self.SpawnerOrigin`))
  (bind (_result _itemtocarry) (`self.IsFrogShouldCarryItem`))
  (if _result
    (`self.AddStaticMeshItem` _itemtocarry))
  (bind _asbp_frog_game_mode (cast `/Game/BP_FrogGameMode` (`GameplayStatics.GetGameMode`)))
  (set `self.SpawnerOrigin` SpawnerOrigin)
  (`/Game/BP_FrogGameMode.AutoRegisterFrog` _asbp_frog_game_mode self)
  (set `self.GameCycleSpeed` (`/Game/BP_FrogGameMode.GameCycleSpeed` _asbp_frog_game_mode))
  (set `self.FrogSpeed` (`/Game/BP_FrogGameMode.FrogSpeed` _asbp_frog_game_mode))
  (bind _splinefound (`self.SetNewSplineToFollow` SplineToFollow))
  (if _splinefound
    (bind _result_2 (`/Engine/EditorBlueprintResources/StandardMacros.IncrementInt` (`/Game/BP_Spawner.CurrentFrogNumber` _spawnerorigin))
      (:`  `
        (set `/Game/BP_Spawner.CurrentFrogNumber` _result_2 _spawnerorigin))))
  (return))

(fn `IsFrogShouldCarryItem`
  (returns (Result :type Boolean) (ItemToCarry :type "StaticMesh Object Reference"))
  (bind _asbp_frog_game_mode (cast `/Game/BP_FrogGameMode` (`GameplayStatics.GetGameMode`)))
  (bind _meshscollected (`/Game/BP_FrogGameMode.MeshsCollected` _asbp_frog_game_mode))
  (bind _returnvalue (`KismetArrayLibrary.Array_IsNotEmpty` _meshscollected))
  (if _returnvalue
    (return _returnvalue (`|GetArrayItem` _meshscollected))))

(fn `KillFrog`
  (bind _spawnerorigin (`self.SpawnerOrigin`))
  (bind _result (`/Engine/EditorBlueprintResources/StandardMacros.DecrementInt` (`/Game/BP_Spawner.CurrentFrogNumber` _spawnerorigin))
    (:`  `
      (set `/Game/BP_Spawner.CurrentFrogNumber` _result _spawnerorigin)
      (bind _asbp_frog_game_mode (cast `/Game/BP_FrogGameMode` (`GameplayStatics.GetGameMode`)))
      (if (`self.IsCarryItem`)
        (`/Game/BP_FrogGameMode.AddItemToCollected` _asbp_frog_game_mode (`self.TransportedMesh`)))
      (bind _success_status (`/Game/BP_FrogGameMode.UnregisterFrog` _asbp_frog_game_mode self))
      (if _success_status
        (`self.K2_DestroyActor`)))))

(fn `SetNewSplineToFollow`
  (params (NewSplineToFollow :type "/Game/BP_Way Object Reference") (StartTime :type "Float (double-precision)"))
  (returns (SplineFound :type Boolean))
  (locals (SplineLength :type "Float (double-precision)"))
  (bind _t_move (`self.T_Move`))
  (set `self.SplineToFollow` NewSplineToFollow)
  (bind _playrate (`self.GetPlayRate`))
  (`TimelineComponent.SetPlayRate` _t_move _playrate)
  (`TimelineComponent.SetNewTime` _t_move StartTime)
  (return (`KismetSystemLibrary.IsValid` NewSplineToFollow)))

(fn `UserConstructionScript`)