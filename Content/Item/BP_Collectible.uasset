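; BP_Collectible is a pickup item that the frog character collects on overlap.
; On BeginPlay it registers itself with BP_FrogGameMode under its sequence index.
; On overlap it passes its mesh to the frog and, if accepted, adds itself to its associated end way's collected list and destroys itself.
; The construction script applies the configured mesh and material to each instance.
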(event `self.ReceiveBeginPlay`
  (bind _asbp_frog_game_mode (cast `/Game/BP_FrogGameMode` (`GameplayStatics.GetGameMode`)))
  (`/Game/BP_FrogGameMode.RegisterCollectible` _asbp_frog_game_mode self (`self.AssociatedSequenceIndex`)))

(event `self.ReceiveActorBeginOverlap`
  (params (OtherActor :type "Actor Object Reference"))
  (bind _asbp_frog (cast `/Game/Frog/BP_Frog` OtherActor))
  (bind _itemwasadd (`/Game/Frog/BP_Frog.AddStaticMeshItem` _asbp_frog (`self.MeshToCollect`)))
  (if _itemwasadd
    (`KismetArrayLibrary.Array_AddUnique` (`/Game/BP_EndWay.ItemCollected` (`self.AssociatedEndWay`)) self)
    (`self.K2_DestroyActor`)))

(fn `UserConstructionScript`
  (bind _itemmesh (`self.ItemMesh`))
  (`StaticMeshComponent.SetStaticMesh` _itemmesh (`self.MeshToCollect`))
  (`PrimitiveComponent.SetMaterial` _itemmesh 0 (`self.MeshMaterial`)))